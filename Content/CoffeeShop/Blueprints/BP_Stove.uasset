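; Stove actor in the coffee shop game that cooks a burger and serves it to the current customer.
; Overlapping InteractZone registers the stove on the third-person character.
; Interact, also exposed through Cook, alternates between spawning a cooking burger and serving it at the exit point.
; Serving raises customer happiness for a perfect burger, damages them for a dangerous one, or otherwise lowers happiness.
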(event `Interact`
  (bind _currentburger (`self.CurrentBurger`))
  (`KismetSystemLibrary.PrintString` "Stove Interacted")
  (if (`KismetSystemLibrary.IsValid` (`self.CurrentBurger`))
    (bind _isperfect (`/Game/CoffeeShop/Blueprints/BP_Burger.IsPerfect` (`self.CurrentBurger`)))
    (if _isperfect
      (`/Game/Characters/Customer.HappinessChange` (`self.CurrentCustomer`) 40)
      (else
        (bind _isdangerous (`/Game/CoffeeShop/Blueprints/BP_Burger.IsDangerous` (`self.CurrentBurger`)))
        (if _isdangerous
          (`GameplayStatics.ApplyDamage` (`self.CurrentCustomer`) 20.0)
          (else
            (`/Game/Characters/Customer.HappinessChange` (`self.CurrentCustomer`) -10)))))
    (`/Game/CoffeeShop/Blueprints/BP_Burger.StopCooking` _currentburger)
    (`self.K2_SetActorLocation` _currentburger (`SceneComponent.K2_GetComponentLocation` (`self.BurgerExitPoint`)) true false)
    (`/Game/Characters/Customer.EatBurger` (`self.CurrentCustomer`))
    (set `self.CurrentBurger` null)
    (set `self.CurrentCustomer` null)
    (else
      (bind _returnvalue (`|SpawnActorFromClass` (`self.BurgerClass`) (`SceneComponent.K2_GetComponentToWorld` (`self.BurgerSpawnPoint`)) "Undefined" "MultiplyWithRoot" null null))
      (bind _output_get (set `self.CurrentBurger` _returnvalue))
      (`/Game/CoffeeShop/Blueprints/BP_Burger.StartCooking` _output_get))))

(event `self.InteractZone.OnComponentBeginOverlap`
  (params (OverlappedComponent :type "PrimitiveComponent Object Reference") (OtherActor :type "Actor Object Reference") (OtherComp :type "PrimitiveComponent Object Reference") (OtherBodyIndex :type Integer) (bFromSweep :type Boolean) (SweepResult :type "HitResult Structure (by ref)"))
  (bind _asbp_third_person_character (cast `/Game/ThirdPerson/Blueprints/BP_ThirdPersonCharacter` OtherActor))
  (set `/Game/ThirdPerson/Blueprints/BP_ThirdPersonCharacter.currentStove` self _asbp_third_person_character))

(event `self.InteractZone.OnComponentEndOverlap`
  (params (OverlappedComponent :type "PrimitiveComponent Object Reference") (OtherActor :type "Actor Object Reference") (OtherComp :type "PrimitiveComponent Object Reference") (OtherBodyIndex :type Integer))
  (bind _asbp_third_person_character (cast `/Game/ThirdPerson/Blueprints/BP_ThirdPersonCharacter` OtherActor))
  (set `/Game/ThirdPerson/Blueprints/BP_ThirdPersonCharacter.currentStove` null _asbp_third_person_character))

(fn `Cook`
  (`self.Interact`))

(fn `UserConstructionScript`)