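; Burger actor for the coffee shop that tracks how long it cooks and rates its doneness from raw to burned.
; StartCooking resets the timer and StopCooking halts it; while cooking, Tick accumulates time, sets a status text by threshold and prints it each frame.
; UpdateVisuals switches on CookState to set the mesh material, but every band writes state 0 and no material is specified in any case.
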(event `self.ReceiveTick`
  (params (DeltaSeconds :type "Float (single-precision)"))
  (if (`self.bIsCooking`)
    (bind _output_get (set `self.CookTime` (+ (`self.CookTime`) DeltaSeconds)))
    (`self.UpdateVisuals` self)
    (if (< _output_get 2.0)
      (bind _output_get_2 (set `self.CookStatusText` "raw"))
      (`KismetSystemLibrary.PrintString` (`KismetTextLibrary.Conv_TextToString` _output_get_2))
      (set `self.CookState` 0)
      (elif (< _output_get 4.0)
        (bind _output_get_3 (set `self.CookStatusText` "undercooked"))
        (`KismetSystemLibrary.PrintString` (`KismetTextLibrary.Conv_TextToString` _output_get_3))
        (set `self.CookState` 0)
        (elif (< _output_get 6.0)
          (bind _output_get_4 (set `self.CookStatusText` "perfect"))
          (`KismetSystemLibrary.PrintString` (`KismetTextLibrary.Conv_TextToString` _output_get_4))
          (set `self.CookState` 0)
          (elif (< _output_get 8.0)
            (bind _output_get_5 (set `self.CookStatusText` "overcooked"))
            (`KismetSystemLibrary.PrintString` (`KismetTextLibrary.Conv_TextToString` _output_get_5))
            (set `self.CookState` 0)
            (else
              (bind _output_get_6 (set `self.CookStatusText` "burned"))
              (`KismetSystemLibrary.PrintString` (`KismetTextLibrary.Conv_TextToString` _output_get_6))
              (set `self.CookState` 0))))))))

(event `StartCooking`
  (set `self.bIsCooking` true)
  (set `self.CookTime` 0.0))

(event `StopCooking`
  (set `self.bIsCooking` false))

(event `UpdateVisuals`
  (switch `|SwitchEnum` (`self.CookState`)
    (:`NewEnumerator0`
      (`PrimitiveComponent.SetMaterial` (`self.StaticMesh2`) 0 null))
    (:`NewEnumerator1`
      (`PrimitiveComponent.SetMaterial` (`self.StaticMesh2`) 0 null))
    (:`NewEnumerator2`
      (`PrimitiveComponent.SetMaterial` (`self.StaticMesh2`) 0 null))
    (:`NewEnumerator3`
      (`PrimitiveComponent.SetMaterial` (`self.StaticMesh2`) 0 null))
    (:`NewEnumerator4`
      (`PrimitiveComponent.SetMaterial` (`self.StaticMesh2`) 0 null))))

(fn `UserConstructionScript`)