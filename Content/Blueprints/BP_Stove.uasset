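; BP_Stove is an interactable stove that spawns and cooks one burger at a time.
; An overlap zone registers the stove with BP_ThirdPersonCharacter on entry and clears it on exit.
; Interact spawns a burger and starts cooking, or stops the current one and moves it to the exit point with a sweep.
; BeginPlay casts the order widget to WBP_OrderDisplay but does nothing with the result.
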(event `Interact`
  (`KismetSystemLibrary.PrintString` "Stove Interacted")
  (if (`KismetSystemLibrary.IsValid` (`self.CurrentBurger`))
    (`/Game/Blueprints/BP_Burger.StopCooking` (`self.CurrentBurger`))
    (`self.K2_SetActorLocation` (`self.CurrentBurger`) (`SceneComponent.K2_GetComponentLocation` (`self.BurgerExitPoint`)) true false)
    (set `self.CurrentBurger` null)
    (else
      (bind _returnvalue (`|SpawnActorFromClass` (`self.BurgerClass`) (`SceneComponent.K2_GetComponentToWorld` (`self.BurgerSpawnPoint`)) "Undefined" "MultiplyWithRoot" null null))
      (bind _output_get (set `self.CurrentBurger` _returnvalue))
      (`/Game/Blueprints/BP_Burger.StartCooking` _output_get))))

(event `self.ReceiveBeginPlay`
  (cast `/Game/_Game/Maps/Bluprints/WBP_OrderDisplay` (`WidgetComponent.GetUserWidgetObject` (`self.OrderWidget`))))

(event `self.InteractZone.OnComponentBeginOverlap`
  (params (OverlappedComponent :type "PrimitiveComponent Object Reference") (OtherActor :type "Actor Object Reference") (OtherComp :type "PrimitiveComponent Object Reference") (OtherBodyIndex :type Integer) (bFromSweep :type Boolean) (SweepResult :type "HitResult Structure (by ref)"))
  (bind _asbp_third_person_character (cast `/Game/CoffeeShop/Demo/ThirdPerson/Blueprints/BP_ThirdPersonCharacter` OtherActor))
  (`/Game/CoffeeShop/Demo/ThirdPerson/Blueprints/BP_ThirdPersonCharacter.SetCurrentStove` _asbp_third_person_character self))

(event `self.InteractZone.OnComponentEndOverlap`
  (params (OverlappedComponent :type "PrimitiveComponent Object Reference") (OtherActor :type "Actor Object Reference") (OtherComp :type "PrimitiveComponent Object Reference") (OtherBodyIndex :type Integer))
  (bind _asbp_third_person_character (cast `/Game/CoffeeShop/Demo/ThirdPerson/Blueprints/BP_ThirdPersonCharacter` OtherActor))
  (`/Game/CoffeeShop/Demo/ThirdPerson/Blueprints/BP_ThirdPersonCharacter.clearCurrentStove` _asbp_third_person_character))

(fn `UserConstructionScript`)