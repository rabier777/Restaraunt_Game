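; BP_Table is an interactable table that holds one object the player puts down or picks up.
; On Interact, a held object becomes PlacedObject if the table is empty, attaches to ObjectPlace keeping its world transform, then moves via MoveComponentTo while the player's grab reference clears.
; An empty-handed player instead grabs the placed object, freeing the table.
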(event `/Game/_Game/Bluprints/Interfaces/BPI_Interactable.Interact`
  (params (Player :type "/Game/_Game/Bluprints/BP_Character Object Reference"))
  (bind (_returnvalue _grabbedobject) (`/Game/_Game/Bluprints/BP_Character.GetGrabbedObject` Player))
  (if _returnvalue
    (`/Engine/EditorBlueprintResources/StandardMacros.IsValid` (`self.PlacedObject`)
      (:`Is Not Valid`
        (bind _output_get (set `self.PlacedObject` _grabbedobject))
        (`self.K2_AttachToComponent` _output_get (`self.ObjectPlace`) "None" "KeepWorld" "KeepWorld" "KeepWorld" true)
        (`KismetSystemLibrary.MoveComponentTo` (`/Game/_Game/Bluprints/Interactable/BP_Grabbable.Root` (`self.PlacedObject`)))
        (set `/Game/_Game/Bluprints/BP_Character.GrabbedObject` null Player)))
    (else
      (`/Engine/EditorBlueprintResources/StandardMacros.IsValid` (`self.PlacedObject`)
        (:`Is Valid`
          (`/Game/_Game/Bluprints/BP_Character.Grab` Player (`self.PlacedObject`))
          (set `self.PlacedObject` null))))))

(fn `UserConstructionScript`)