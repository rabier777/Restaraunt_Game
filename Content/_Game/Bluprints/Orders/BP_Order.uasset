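; BP_Order is a single cooking order built around a recipe, tracking its time limit and outcome.
; Activation starts a timer from the recipe's cook time, with a short follow-up timer after it, and dispatchers report time-up, failure and completion.
; TryFinish compares submitted ingredients to the recipe, returning true even on failure.
; Helpers format name and remaining time, and expand recipe amounts into ingredient objects.
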(event `ActivateOrder`
  (`KismetSystemLibrary.K2_SetTimer` null (`self.MainTimerFunction`) (`/Game/_Game/Blueprints/AssetTypes/DA_Recipes_BP.CookTime` (`self.Recipe`))))

(event `MainTimerFinished`
  (`self.OnMainTimeFinished` self)
  (`KismetSystemLibrary.K2_SetTimerDelegate` (`|CreateDelegate` :!event `TimeExpired`) 5.0))

(event `TimeExpired`
  (`self.OnOrderFailed` self)
  (`self.UnbindAllDispatchers`))

(fn `GetOrderIngredients`
  (returns (`Order Ingredients` :type "Array of /Game/_Game/Blueprints/Orders/BP_OrderIngredient Object Reference"))
  (locals (Ingredients :type "Array of /Game/_Game/Blueprints/Orders/BP_OrderIngredient Object Reference"))
  (bind (_keypin _valuepin) (`|MapForEach` (`/Game/_Game/Blueprints/AssetTypes/DA_Recipes_BP.Ingredient` (`self.Recipe`)))
    (:`then`
      (for _ (range 1 (+ (`.Amount_4_81E109773043537F64F88CB24D9C3EB8` (break `/Game/_Game/Blueprints/Structures/BPS_RecipeIngredients` _valuepin)) 1))
        (bind _returnvalue (`|GenericCreateObject` "/Game/_Game/Blueprints/Orders/BP_OrderIngredient.BP_OrderIngredient_C" (`|MakeArray` _keypin)))
        (`KismetArrayLibrary.Array_Add` (`local.Ingredients`) _returnvalue)))
    (:`CompletedPin`
      (return (`local.Ingredients`)))))

(fn `ToText`
  (returns (Text :type Text))
  (locals (Ingredients :type "Array of /Game/_Game/Blueprints/Orders/BP_OrderIngredient Object Reference"))
  (return (`|FormatText` "{name} ({time})" (`KismetSystemLibrary.GetDisplayName` (`self.Recipe`)) (`KismetSystemLibrary.K2_GetTimerRemainingTime` null (`self.MainTimerFunction`)))))

(fn `TryFinish`
  (params (Ingredients :type "Map of /Game/_Game/Blueprints/AssetTypes/DA_FoodItem_BP Object Reference to /Game/_Game/Blueprints/Structures/BPS_RecipeIngredients Structure"))
  (returns (Finished :type Boolean))
  (bind _equal (`/Game/_Game/Blueprints/AssetTypes/DA_Recipes_BP.Compare` (`self.Recipe`) Ingredients))
  (if _equal
    (`self.OnOrderFinished` self)
    (`self.UnbindAllDispatchers`)
    (return true)
    (else
      (`self.OnOrderFailed` self)
      (return true))))

(fn `UnbindAllDispatchers`
  (clear `self.OnMainTimeFinished`)
  (clear `self.OnOrderFailed`)
  (clear `self.OnOrderFinished`))