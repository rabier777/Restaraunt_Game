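; Interactable weapon pickup Blueprint whose WeaponNum selects a knife, pistol or rifle.
; The construction script assigns the matching static mesh and Info text, then enables physics simulation on the mesh.
; LookAtMe writes a weapon description into the passed ItemInfo widget's text block from its own hard-coded strings rather than Info, with an error string for unhandled numbers.
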(fn `LookAtMe`
  (params (`Item Info` :type "/Game/_Game/Blueprints/HUD/Widgets/ItemInfoBP Object Reference"))
  (bind _textblock_0 (`/Game/_Game/Blueprints/HUD/Widgets/ItemInfoBP.TextBlock_0` `Item Info`))
  (switch `int` (`self.WeaponNum`)
    (:`Default`
      (set `TextBlock.Text` "ERROR: Missing description" _textblock_0))
    (:`0`
      (set `TextBlock.Text` "Knife - melee" _textblock_0))
    (:`1`
      (set `TextBlock.Text` "Handgun - ranged" _textblock_0))
    (:`2`
      (set `TextBlock.Text` "Rifle - ranged" _textblock_0))))

(fn `UserConstructionScript`
  (bind _staticmesh (`self.StaticMesh`))
  (switch `int` (`self.WeaponNum`)
    (:`0`
      (`StaticMeshComponent.SetStaticMesh` _staticmesh "/Game/_Game/Assets/Weapons/SM_Knife_01.SM_Knife_01")
      (set `self.Info` "Knife - melee"))
    (:`1`
      (`StaticMeshComponent.SetStaticMesh` _staticmesh "/Game/_Game/Assets/Weapons/SM_Weapons_03_MERGED.SM_Weapons_03_MERGED")
      (set `self.Info` "Pistol - ranged"))
    (:`2`
      (`StaticMeshComponent.SetStaticMesh` _staticmesh "/Game/_Game/Assets/Weapons/SM_Weapons_04_MERGED.SM_Weapons_04_MERGED")
      (set `self.Info` "Rifle - ranged")))
  (`PrimitiveComponent.SetSimulatePhysics` (`self.StaticMesh`) true))