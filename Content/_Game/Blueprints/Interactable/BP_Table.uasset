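; BP_Table is an interactable table that stores one object the player is carrying.
; On Interact, a held object goes onto the table if it is empty: it attaches to ObjectPlace keeping its world transform, then moves via MoveComponentTo, and the player's grab reference clears.
; An empty-handed Interact makes the player grab the placed object and frees the table.
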(event `/Game/_Game/Blueprints/Interfaces/BPI_Interactable.Interact`
  (params (Player :type "Object Object Reference"))
  (bind (_returnvalue _grabbedobject) (`self.GetGrabbedObject` Player))
  (if _returnvalue
    (`/Engine/EditorBlueprintResources/StandardMacros.IsValid` (`self.PlacedObject`)
      (:`Is Not Valid`
        (bind _output_get (set `self.PlacedObject` _grabbedobject))
        (`self.K2_AttachToComponent` _output_get (`self.ObjectPlace`) "None" "KeepWorld" "KeepWorld" "KeepWorld" true)
        (`KismetSystemLibrary.MoveComponentTo` (`/Game/_Game/Blueprints/Interactable/BP_Grabbable.Root` (`self.PlacedObject`)))
        (set `/Game/_Game/Blueprints/Interactable/BP_Table.GrabbedObject` null Player)))
    (else
      (`/Engine/EditorBlueprintResources/StandardMacros.IsValid` (`self.PlacedObject`)
        (:`Is Valid`
          (`self.Grab` Player (`self.PlacedObject`))
          (set `self.PlacedObject` null))))))

(fn `UserConstructionScript`)