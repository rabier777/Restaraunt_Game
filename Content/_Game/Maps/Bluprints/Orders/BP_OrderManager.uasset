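; BP_OrderManager generates and tracks active recipe orders up to a maximum count.
; A looping timer adds BP_Order objects with random recipes, stops at the cap, and restarts when an order finishes or fails.
; Submitted ingredients are offered to each order until one accepts them.
; Order delegates report main-timer expiry, failure and completion as colored debug prints, while Tick prints the active list.
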(event `self.ReceiveTick`
  (params (DeltaSeconds :type "Float (single-precision)"))
  (`self.PrintTasks` DeltaSeconds))

(event `self.ReceiveBeginPlay`
  (`self.AddTask`)
  (`self.StartAddTaskTimer`))

(event `StartAddTaskTimer`
  (bind _returnvalue (`KismetSystemLibrary.K2_SetTimerDelegate` (`|CreateDelegate` :!event `AddTask`) (`self.NextTaskDelay`) true))
  (set `self.AddTaskTimerHandle` _returnvalue))

(event `AddTask`
  (if (== (`KismetArrayLibrary.Array_Length` (`self.Tasks`)) (`self.MaxTaskAmount`))
    (`KismetSystemLibrary.K2_ClearAndInvalidateTimerHandle` (`self.AddTaskTimerHandle`))
    (else
      (bind _order (`self.InitTask` (`KismetArrayLibrary.Array_Random` (`self.Recipes`))))
      (`KismetArrayLibrary.Array_Add` (`self.Tasks`) _order))))

(event `TryFinishTask`
  (params (Ingredients :type "Map of /Game/_Game/Maps/Bluprints/AssetTypes/DA_FoodItem_BP Object Reference to /Game/_Game/Maps/Bluprints/Structures/BPS_RecipeIngredients Structure"))
  (for _array_element (`self.Tasks`)
    (bind _finished (`/Game/_Game/Maps/Bluprints/Orders/BP_Order.TryFinish` _array_element Ingredients))
    (if _finished
      (break))))

(event `StartAddTimerIfNeeded`
  (if (not (`KismetSystemLibrary.K2_IsValidTimerHandle` (`self.AddTaskTimerHandle`)))
    (`self.StartAddTaskTimer`)))

(event `OrderMainTimerFinished`
  (params (Order :type "/Game/_Game/Maps/Bluprints/Orders/BP_Order Object Reference"))
  (`KismetSystemLibrary.PrintString` (`KismetSystemLibrary.GetDisplayName` (`/Game/_Game/Maps/Bluprints/Orders/BP_Order.Recipe` Order)) true true (struct :`R` 1.0 :`G` 0.407114 :`A` 1.0)))

(event `OrderFailed`
  (params (Order :type "/Game/_Game/Maps/Bluprints/Orders/BP_Order Object Reference"))
  (`KismetSystemLibrary.PrintString` (`KismetSystemLibrary.GetDisplayName` (`/Game/_Game/Maps/Bluprints/Orders/BP_Order.Recipe` Order)) true true (struct :`R` 1.0 :`B` 0.023705 :`A` 1.0))
  (`KismetArrayLibrary.Array_RemoveItem` (`self.Tasks`) Order)
  (`self.StartAddTimerIfNeeded`))

(event `OrderFinished`
  (params (Order :type "/Game/_Game/Maps/Bluprints/Orders/BP_Order Object Reference"))
  (`KismetSystemLibrary.PrintString` (`KismetSystemLibrary.GetDisplayName` (`/Game/_Game/Maps/Bluprints/Orders/BP_Order.Recipe` Order)) true true (struct :`R` 0.003124 :`G` 1.0 :`B` 0.078345 :`A` 1.0))
  (`KismetArrayLibrary.Array_RemoveItem` (`self.Tasks`) Order)
  (`self.StartAddTimerIfNeeded`))

(fn `InitTask`
  (params (Recipe :type "/Game/_Game/Maps/Bluprints/AssetTypes/DA_Recipes_BP Object Reference"))
  (returns (Order :type "/Game/_Game/Maps/Bluprints/Orders/BP_Order Object Reference"))
  (bind _returnvalue (`|GenericCreateObject` "/Game/_Game/Maps/Bluprints/Orders/BP_Order.BP_Order_C" Recipe))
  (add `/Game/_Game/Maps/Bluprints/Orders/BP_Order.OnMainTimeFinished` _returnvalue (`|CreateDelegate` :!event `OrderMainTimerFinished`))
  (add `/Game/_Game/Maps/Bluprints/Orders/BP_Order.OnOrderFailed` _returnvalue (`|CreateDelegate` :!event `OrderFailed`))
  (add `/Game/_Game/Maps/Bluprints/Orders/BP_Order.OnOrderFinished` _returnvalue (`|CreateDelegate` :!event `OrderFinished`))
  (`/Game/_Game/Maps/Bluprints/Orders/BP_Order.ActivateOrder` _returnvalue)
  (return _returnvalue))

(fn `PrintTasks`
  (params (DeltaTime :type "Float (double-precision)"))
  (locals (Text :type Text))
  (for _array_element (`self.Tasks`)
    (set `local.Text` (`|FormatText` "{Text}|{Name}" (`local.Text`) (`/Game/_Game/Maps/Bluprints/Orders/BP_Order.ToText` _array_element))))
  (`KismetSystemLibrary.PrintText` (`local.Text`) true true (struct :`G` 0.66 :`B` 1.0 :`A` 1.0) (`local.DeltaTime`)))

(fn `UserConstructionScript`)