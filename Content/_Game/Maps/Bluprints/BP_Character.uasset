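; Player character Blueprint that handles interacting with the world and carrying a single object.
; On interact input, a short vertical sphere trace just ahead, ignoring the held object, sends InteractMessage to the hit actor with the character as argument.
; If nothing is hit, it drops and clears any held object.
; The Grab event stores an object, attaches it to Hands keeping world transform, then moves it to the attachment origin with MoveComponentTo.
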(event `EnhancedInput|/Game/_Game/Inputs/IA_Interact`
  (params (ActionValue :type Boolean) (ElapsedSeconds :type "Float (double-precision)") (TriggeredSeconds :type "Float (double-precision)") (InputAction :type "InputAction Object Reference" :default "/Game/_Game/Inputs/IA_Interact.IA_Interact"))
  (bind (_returnvalue _grabbedobject) (`self.GetGrabbedObject`))
  (bind _x (.x (+ (* (`self.GetActorForwardVector`) 50.0) (`self.K2_GetActorLocation`))))
  (bind _y (.y (+ (* (`self.GetActorForwardVector`) 50.0) (`self.K2_GetActorLocation`))))
  (bind _z (.z (+ (* (`self.GetActorForwardVector`) 50.0) (`self.K2_GetActorLocation`))))
  (:`Started`
    (bind (_outhit _returnvalue_2) (`KismetSystemLibrary.SphereTraceSingle` (`KismetMathLibrary.MakeVector` _x _y (+ _z -50.0)) (`KismetMathLibrary.MakeVector` _x _y (+ _z 10.0)) 30.0 "TraceTypeQuery3" false (`|MakeArray` (`self.GrabbedObject`) :!type "Actor Object Reference") "ForDuration"))
    (if _returnvalue_2
      (message `/Game/_Game/Maps/Bluprints/Interfaces/BPI_Interactable.Interact` (`.HitActor` (`GameplayStatics.BreakHitResult` _outhit)) self)
      (elif _returnvalue
        (`/Game/_Game/Maps/Bluprints/Interactable/BP_Grabbable.Drop` _grabbedobject)
        (set `self.GrabbedObject` null)))))

(event `Grab`
  (params (ObjectGrab :type "/Game/_Game/Maps/Bluprints/Interactable/BP_Grabbable Object Reference"))
  (bind _output_get (set `self.GrabbedObject` ObjectGrab))
  (`self.K2_AttachToComponent` _output_get (`self.Hands`) "None" "KeepWorld" "KeepWorld" "KeepWorld" true)
  (`KismetSystemLibrary.MoveComponentTo` (`Actor.RootComponent` (`self.GrabbedObject`))))

(fn `GetGrabbedObject`
  (returns (ReturnValue :type Boolean) (GrabbedObject :type "/Game/_Game/Maps/Bluprints/Interactable/BP_Grabbable Object Reference"))
  (bind _grabbedobject (`self.GrabbedObject`))
  (return (`KismetSystemLibrary.IsValid` _grabbedobject) _grabbedobject))

(fn `UserConstructionScript`)